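; GlooBlob_BP is a blob actor that animates itself in when spawned, growing and shifting color.
; On BeginPlay it picks a random small size multiplier and plays a grow timeline that drives the static mesh's uniform world scale.
; Half a second later it creates a dynamic material instance on the mesh and plays a color timeline that drives its ColorLerp parameter.
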(event `self.ReceiveBeginPlay`
  (`|ExecutionSequence`
    (:`then_0`
      (set `self.RandomSizeMultiplier` (`KismetMathLibrary.RandomFloatInRange` 0.05 0.13)))
    (:`then_1`
      ;[1 1 1] Grow
      (bind (_direction _scale) (`Timeline|Grow_Timeline`)
        (:`Update`
          (`SceneComponent.SetWorldScale3D` (`self.StaticMesh`) (`KismetMathLibrary.Conv_DoubleToVector` (* _scale (`self.RandomSizeMultiplier`)))))))
    (:`then_2`
      (`KismetSystemLibrary.Delay` 0.5)
      (bind _returnvalue (`PrimitiveComponent.CreateDynamicMaterialInstance` (`self.StaticMesh`) 0 null "None"))
      (bind (_direction_2 _color_lerp) (`Timeline|Color_Timeline`)
        (:`Update`
          (`MaterialInstanceDynamic.SetScalarParameterValue` _returnvalue "ColorLerp" _color_lerp))))))

(fn `UserConstructionScript`)